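; Solar panel component that simulates power generation from the SunSky sun, displays it and logs it to CSV.
; Every tick it gathers the owner's "cell" meshes and line-traces from a distant sun point to each.
; Clear cells receive power from an incidence-angle formula using panel roll and assumed constants; blocked cells scale it by the occluder material's Opacity.
; Summed power is recorded with date and game time to a hardcoded file path.
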(event EventBeginPlay
  (Utilities|Time|SetTimerbyFunctionName 0 "Timer" 1.0 true)
  (CallFunction|FindSun)
  (CallFunction|FindCellsinActor)
  (CallFunction|CalculateMaxPower)
  (CallFunction|CalculateGeneratedPower)
  (CallFunction|DisplayGeneratedPower)
  (bind _energydataset (CallFunction|RecordData (Variables|Default|GetGeneratedPower)))
  (CallFunction|SavetoFile _energydataset))

(event EventTick
  (params (DeltaSeconds :type Float%20%28single-precision%29))
  (CallFunction|FindSun)
  (CallFunction|FindCellsinActor)
  (CallFunction|CalculateMaxPower)
  (CallFunction|CalculateGeneratedPower)
  (CallFunction|DisplayGeneratedPower)
  (bind _energydataset (CallFunction|RecordData (Variables|Default|GetGeneratedPower)))
  (CallFunction|SavetoFile _energydataset))

(fn FindSun
  (bind _returnvalue (Actor|GetActorOfClass "/SunPosition/SunSky.SunSky_C"))
  (Variables|Default|SetsunLocation (* (Math|Vector|GetForwardVector (Transformation|GetWorldRotation (Variables|/SunPosition/SunSky.SunSky_C|GetDirectionalLight _returnvalue))) (Variables|Default|GetTakingSunToAfar))))

(fn FindCellsinActor
  (Utilities|Array|Clear (Variables|Default|GetCells))
  (for _array_element (Actor|GetComponentsByClass (Components|GetOwner) "/Script/Engine.StaticMeshComponent")
    (if (Utilities|String|StartsWith (Utilities|GetObjectName _array_element) "cell")
      (Utilities|Array|AddUnique (Variables|Default|GetCells) _array_element))))

(fn CalculateMaxPower
  (bind _powergenbasedonsunloc (CallFunction|SolarEnergyCalculaterBasedonLocation (Variables|Default|GetsunLocation)))
  (Variables|Default|SetMaxPower (* (* _powergenbasedonsunloc (Utilities|Array|Length (Variables|Default|GetCells))) (Variables|Default|GetTime%20Factor%20%28Hours%29))))

(fn CalculateGeneratedPower
  (for _array_element (Variables|Default|GetCells)
    (bind _generatedpower (CallFunction|CalculateCellPower (Transformation|GetWorldLocation _array_element)))
    (LocalVariables|SetpCurrentPower (+ _generatedpower (LocalVariables|GetpCurrentPower))))
  (Variables|Default|SetGeneratedPower (LocalVariables|GetpCurrentPower)))

(fn CalculateCellPower
  (params (cellPosition :type Vector))
  (bind _sunlocation (Variables|Default|GetsunLocation))
  (LocalVariables|SetpCurrentCellPosition cellPosition)
  (bind (_outhit _returnvalue) (Collision|LineTraceByChannel _sunlocation (LocalVariables|GetpCurrentCellPosition) "TraceTypeQuery3" false 0 "ForDuration" true "(R=1.000000,G=0.834536,B=0.000000,A=1.000000)" "(R=1.000000,G=0.099408,B=0.000000,A=1.000000)" 0.1))
  (bind _powergenbasedonsunloc (CallFunction|SolarEnergyCalculaterBasedonLocation _sunlocation))
  (if _returnvalue
    ;[1 1 1] OTHER SURFACE HIT
    (if (.bBlockingHit (Collision|BreakHitResult _outhit))
      (bind _asmaterial_instance (Utilities|Casting|CastToMaterialInstance (Rendering|Material|GetMaterial (.HitComponent (Collision|BreakHitResult _outhit)) 0)))
      (for _array_element (Variables|/Script/Engine.MaterialInstance|GetScalarParameterValues _asmaterial_instance)
        (if (== (.name (.parameterinfo _array_element)) "Opacity")
          (if (>= _powergenbasedonsunloc 0.0)
            (return (* (- 1.0 (.parametervalue _array_element)) (* _powergenbasedonsunloc (Variables|Default|GetTime%20Factor%20%28Hours%29))))
            (else
              (return 0.0)))))
      (else
        (return 0.0)))
    (else
      ;[1 1 1] SOLAR PANEL HIT
      (Rendering|Debug|DrawDebugLine _sunlocation (LocalVariables|GetpCurrentCellPosition) "(R=1.000000,G=0.766024,B=0.241486,A=1.000000)" 0.0 0.0)
      (return (* _powergenbasedonsunloc (Variables|Default|GetTime%20Factor%20%28Hours%29))))))

(fn DisplayGeneratedPower
  (Rendering|Debug|DrawDebugString (Transformation|GetActorLocation (Components|GetOwner)) (Utilities|String|Append "Power " (Utilities|String|ToString(Float) (Variables|Default|GetGeneratedPower))) 0 "(R=1.000000,G=1.000000,B=1.000000,A=1.000000)"))

(fn SolarEnergyCalculaterBasedonLocation
  (params (SunLoc :type Vector))
  (bind _returnvalue (Math|Conversions|ToTransform(Vector) SunLoc))
  (bind (_azimuth _elevation) (Class|KismetMathLibrary|GetAzimuthandElevation SunLoc _returnvalue))
  (bind _returnvalue_2 (- 9e+01 _elevation))
  ;[1 1 1] Solar Radiation (Earth to sun distance, surface tilt, Solar constant has set to assumed values)
  (bind _returnvalue_3 (Actor|GetActorOfClass "/Game/SolarPanelActors/BP_SolarPanel.BP_SolarPanel_C"))
  (return (* (LocalVariables|GetSolarPanelArea%28AssumedConst%29) (/ (* (+ (* (Math|Trig|Sin(Degrees) _returnvalue_2) (Math|Trig|Sin(Degrees) (.roll (Transformation|GetActorRotation _returnvalue_3))) (Math|Trig|Cos(Degrees) (- _azimuth (LocalVariables|GetSurface%20Direction%20%28Surface%20Azimuth%29)))) (* (Math|Trig|Cos(Degrees) _returnvalue_2) (Math|Trig|Cos(Degrees) (.roll (Transformation|GetActorRotation _returnvalue_3))))) (LocalVariables|GetSolarConstant%20%28Gsc%29)) (Math|Float|Power (LocalVariables|GetDistance%20to%20sun%20in%20Astronomica%20units) 2.0)) (LocalVariables|GetSolar%20Panel%20Yield%28AssumedConst%29) (LocalVariables|GetPerformance%20Ratio%28Assumed%20Const%29))))

(fn SavetoFile
  (params (GeneratedPowerDataInput :type Array%20of%20Strings))
  (for _array_element GeneratedPowerDataInput
    (LocalVariables|SetData%20String (Utilities|String|Append (LocalVariables|GetData%20String) (Utilities|String|Append _array_element ", 
"))))
  (Class|ReadWritePluginBPLibrary|SaveStringtoFile "C:\\Users\\Madara\\Documents\\Unreal Projects\\PhD_Experiment\\GeneratedDataCSV\\Data.CSV" (LocalVariables|GetData%20String)))

(fn Timer
  (bind _output_get (Variables|Default|SetCounter (+ (Variables|Default|GetCounter) 1)))
  (return _output_get))

(fn RecordData
  (params (GeneratedPower :type Float%20%28double-precision%29))
  (bind _dataarray_new (Variables|Default|GetDataArray_New))
  (bind _returnvalue (Actor|GetActorOfClass "/SunPosition/SunSky.SunSky_C"))
  ;[1 1 1] Integer counter
  (bind _timeinsecondsfromstart (CallFunction|Timer))
  (Utilities|Array|Add _dataarray_new (Utilities|String|Append (Utilities|String|Append "2023" "/" (Utilities|String|ToString(Integer) (Variables|/SunPosition/SunSky.SunSky_C|GetMonth _returnvalue)) "/" (Utilities|String|ToString(Integer) (Variables|/SunPosition/SunSky.SunSky_C|GetDay _returnvalue))) "," (Utilities|String|ToString(Float) (Actor|GetGameTimeSinceCreation _returnvalue)) "," (Utilities|String|ToString(Float) GeneratedPower)))
  (Utilities|Array|SetArrayElem _dataarray_new _timeinsecondsfromstart (Utilities|String|Append (Utilities|String|Append "2023" "/" (Utilities|String|ToString(Integer) (Variables|/SunPosition/SunSky.SunSky_C|GetMonth _returnvalue)) "/" (Utilities|String|ToString(Integer) (Variables|/SunPosition/SunSky.SunSky_C|GetDay _returnvalue))) "," (Utilities|String|ToString(Float) (Actor|GetGameTimeSinceCreation _returnvalue)) "," (Utilities|String|ToString(Float) GeneratedPower)) true)
  (return (Variables|Default|GetDataArray_New)))